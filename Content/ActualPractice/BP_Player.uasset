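; BP_Player is the player in a simple shooter, moving on input, auto-firing bullets and destroying what it touches.
; BeginPlay registers Enhanced Input, starts a looping timer that spawns BP_Bullet at the player's transform, and creates the WBP_Main HUD.
; Tick moves it kinematically (P = P0 + vt) from input axes without sweeping.
; Box overlaps explode and destroy the other actor, while AddCount increments the HUD's removal counter.
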(event `self.ReceiveBeginPlay`
  ;[1 1 1] Input 초기 설정
  (`EnhancedInputSubsystemInterface.AddMappingContext` (pcsubsystem `EnhancedInputLocalPlayerSubsystem` (`GameplayStatics.GetPlayerController` 0)) "/Game/ActualPractice/InputMapping.InputMapping" 0 (struct))
  (`KismetSystemLibrary.K2_SetTimer` null "CreateBullet" 0.5 true)
  (bind _returnvalue (`|CreateWidget` "/Game/ActualPractice/WBP_Main.WBP_Main_C"))
  (bind _output_get (set `self.MainWidget` _returnvalue))
  (`UserWidget.AddToViewport` _output_get 0))

(event `self.ReceiveTick`
  (params (DeltaSeconds :type "Float (single-precision)"))
  (`self.K2_SetActorLocation` (+ (* (* (+ (* (`self.GetActorRightVector`) (`|GetInputActionValue`)) (* (`self.GetActorForwardVector`) (`|GetInputActionValue`))) (`self.Speed`)) DeltaSeconds) (`self.K2_GetActorLocation`))))

(event `self.Box.OnComponentBeginOverlap`
  (params (OverlappedComponent :type "PrimitiveComponent Object Reference") (OtherActor :type "Actor Object Reference") (OtherComp :type "PrimitiveComponent Object Reference") (OtherBodyIndex :type Integer) (bFromSweep :type Boolean) (SweepResult :type "HitResult Structure (by ref)"))
  (`|ExecutionSequence`
    (:`then_0`
      (`GameplayStatics.SpawnEmitterAtLocation` "/Game/StarterContent/Particles/P_Explosion.P_Explosion" (`self.K2_GetActorLocation` OtherActor)))
    (:`then_1`
      ;[1 1 1] 부딪힌 액터 파괴
      (`self.K2_DestroyActor` OtherActor))))

(fn `Add Count`
  (bind _output_get (set `self.RemoveCount` (+ (`self.RemoveCount`) 1)))
  (`TextBlock.SetText` (`/Game/ActualPractice/WBP_Main.RemoveCount` (`self.MainWidget`)) (`KismetTextLibrary.Conv_IntToText` _output_get)))

(fn `CreateBullet`
  (`|SpawnActorFromClass` "/Game/ActualPractice/BP_Bullet.BP_Bullet_C" (`self.GetTransform`) "Undefined" "MultiplyWithRoot" null null))

(fn `UserConstructionScript`)