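; BP_Floor is a scrolling floor actor that moves continuously and loops to create endless ground.
; Each Tick moves it opposite its forward vector at ScrollSpeed, scaled by delta time.
; After that move, it jumps ahead along world X by a fixed span once it passes a negative X threshold, recycling the same piece.
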(event `self.ReceiveTick`
  (params (DeltaSeconds :type "Float (single-precision)"))
  (bind _returnvalue_x (`KismetMathLibrary.BreakVector` (`self.K2_GetActorLocation`)))
  (`|ExecutionSequence`
    (:`then_0`
      (`self.K2_SetActorLocation` (+ (* (* (* (`self.GetActorForwardVector`) -1.0) (`self.ScrollSpeed`)) DeltaSeconds) (`self.K2_GetActorLocation`))))
    (:`then_1`
      (if (< _returnvalue_x -8000.0)
        (`self.K2_SetActorLocation` (+ (`self.K2_GetActorLocation`) (16000.0 0.0 0.0)))))))

(fn `UserConstructionScript`)