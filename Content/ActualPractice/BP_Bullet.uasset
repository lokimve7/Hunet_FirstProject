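; BP_Bullet is a projectile actor that destroys whatever it overlaps and credits the player.
; Each tick it moves itself along its forward vector at Speed, using a non-swept SetActorLocation.
; When its StaticMesh begins an overlap, it destroys the other actor without any type check, plays an explosion sound, calls AddCount on the first BP_Player found, then destroys itself.
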(event `self.ReceiveTick`
  (params (DeltaSeconds :type "Float (single-precision)"))
  (`self.K2_SetActorLocation` (+ (* (* (`self.GetActorForwardVector`) (`self.Speed`)) DeltaSeconds) (`self.K2_GetActorLocation`))))

(event `self.StaticMesh.OnComponentBeginOverlap`
  (params (OverlappedComponent :type "PrimitiveComponent Object Reference") (OtherActor :type "Actor Object Reference") (OtherComp :type "PrimitiveComponent Object Reference") (OtherBodyIndex :type Integer) (bFromSweep :type Boolean) (SweepResult :type "HitResult Structure (by ref)"))
  (`self.K2_DestroyActor` OtherActor)
  (`GameplayStatics.PlaySound2D` "/Game/StarterContent/Audio/Explosion01.Explosion01" 1.0 1.0 0.0 null null)
  (bind _returnvalue (`GameplayStatics.GetActorOfClass` "/Game/ActualPractice/BP_Player.BP_Player_C"))
  (`/Game/ActualPractice/BP_Player.Add Count` _returnvalue)
  (`self.K2_DestroyActor`))

(fn `UserConstructionScript`)