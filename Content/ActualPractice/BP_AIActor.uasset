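; BP_AIActor is a practice AI actor that flies in a straight line toward where the player was at spawn.
; BeginPlay finds BP_Player and caches the normalized direction to it once, so the actor does not home in afterward.
; Tick moves it along that direction by Speed scaled with delta time, without sweep.
; Its Sphere prints the other actor's name with a Korean message when an overlap ends.
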(event `self.ReceiveBeginPlay`
  (`|ExecutionSequence`
    (:`then_0`
      ;[1 1 1] 플레이어를 찾자
      (bind _returnvalue (`GameplayStatics.GetActorOfClass` "/Game/ActualPractice/BP_Player.BP_Player_C"))
      (set `self.Player` _returnvalue))
    (:`then_1`
      ;[0.2282 0.2508 1] 내가 플레이어를 향하는 방향
      (set `self.Dir` (`KismetMathLibrary.Normal` (- (`self.K2_GetActorLocation` (`self.Player`)) (`self.K2_GetActorLocation`)))))))

(event `self.ReceiveTick`
  (params (DeltaSeconds :type "Float (single-precision)"))
  (`self.K2_SetActorLocation` (+ (* (* (`self.Dir`) (`self.Speed`)) DeltaSeconds) (`self.K2_GetActorLocation`))))

(event `self.Sphere.OnComponentBeginOverlap`
  (params (OverlappedComponent :type "PrimitiveComponent Object Reference") (OtherActor :type "Actor Object Reference") (OtherComp :type "PrimitiveComponent Object Reference") (OtherBodyIndex :type Integer) (bFromSweep :type Boolean) (SweepResult :type "HitResult Structure (by ref)")))

(event `self.Sphere.OnComponentEndOverlap`
  (params (OverlappedComponent :type "PrimitiveComponent Object Reference") (OtherActor :type "Actor Object Reference") (OtherComp :type "PrimitiveComponent Object Reference") (OtherBodyIndex :type Integer))
  (`KismetSystemLibrary.PrintString` (`KismetStringLibrary.Concat_StrStr` (`KismetSystemLibrary.GetDisplayName` OtherActor) "와 충돌이 끝남!!")))

(fn `UserConstructionScript`)