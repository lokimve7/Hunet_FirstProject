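; BP_AIActorManager is a spawner that repeatedly creates BP_AIActor instances at its own location.
; Tick runs a Delay of CreateTime before calling CreateAIActor, so the latent node ignores re-triggers while counting and paces the spawns.
; Two unconnected alternatives remain in the graph and never run: a looping timer by function name and a manual DeltaSeconds accumulator.
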(event `self.ReceiveBeginPlay`)

(event `self.ReceiveTick`
  (params (DeltaSeconds :type "Float (single-precision)"))
  (`KismetSystemLibrary.Delay` (`self.CreateTime`))
  (`self.CreateAIActor`))

(fn `CreateAIActor`
  (`|SpawnActorFromClass` "/Game/ActualPractice/BP_AIActor.BP_AIActor_C" (`KismetMathLibrary.MakeTransform` (`self.K2_GetActorLocation`)) "Undefined" "MultiplyWithRoot" null null))

(fn `UserConstructionScript`)